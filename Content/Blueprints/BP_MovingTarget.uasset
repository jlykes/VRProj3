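; BP_MovingTarget is a shootable target that moves along the world X axis and opens a linked BP_DoorTargetActivated on its fifth hit.
; A timeline started at BeginPlay offsets it from its starting location.
; Each trace hit increments a counter shown on the Points text and replays an alpha timeline that drives the sphere material's color lerp.
; The construction script creates that dynamic material with two configurable colors.
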(event EventBeginPlay
  (Utilities|FlowControl|Sequence
    (:then_0
      (Variables|Default|SetOriginalLocation (Transformation|GetActorLocation)))
    (:then_1
      (bind _xpos (Timeline|Location%20timeline Play)
        (:Update
          (Transformation|SetActorLocation (Math|Vector|MakeVector (+ _xpos (.x (Variables|Default|GetOriginalLocation))) (.y (Variables|Default|GetOriginalLocation)) (.z (Variables|Default|GetOriginalLocation))) false))))))

(event EventActorBeginOverlap
  (params (OtherActor :type Actor%20Object%20Reference)))

(event EventTick
  (params (DeltaSeconds :type Float%20%28single-precision%29)))

(event EventTraceHitActorwithComponent
  (params (Component :type Primitive%20Component%20Object%20Reference))
  (Utilities|FlowControl|Sequence
    (:then_0
      (bind _alpha (Timeline|AlphaTimeline PlayFromStart)
        (:Update
          (bind _asmaterial_instance_dynamic (Utilities|Casting|CastToMaterialInstanceDynamic (Rendering|Material|GetMaterial (Variables|Default|GetSphere) 0)))
          (Rendering|Material|SetScalarParameterValue _asmaterial_instance_dynamic "LerpAlpha" _alpha :!class /Script/Engine.MaterialInstanceDynamic))))
    (:then_1
      (bind _output_get (Variables|Default|SetHitCount (+ (Variables|Default|GetHitCount) 1)))
      (Rendering|Components|TextRender|SetText (Variables|Default|GetPoints) (Utilities|String|ToString(Integer) _output_get))
      (if (== (Variables|Default|GetHitCount) 5)
        (bind _asbp_door_target_activated (Utilities|Casting|CastToBP_DoorTargetActivated (Variables|Default|GetDoor)))
        (Default|EventOpen _asbp_door_target_activated)))))

(fn ConstructionScript
  (CallFunction|CreateDMI (Variables|Default|GetSphere) (Variables|Default|GetColor1) (Variables|Default|GetColor2)))

(fn CreateDMI
  (params (SM :type Static%20Mesh%20Component%20Object%20Reference) (Color :type Linear%20Color%20Structure) (Alternate%20Color :type Linear%20Color%20Structure))
  (bind _returnvalue (Rendering|Material|CreateDynamicMaterialInstance SM 0 (Rendering|Material|GetMaterial SM 0) :!class /Script/Engine.PrimitiveComponent))
  (Rendering|Material|SetVectorParameterValue _returnvalue "BaseColor" Color :!class /Script/Engine.MaterialInstanceDynamic)
  (Rendering|Material|SetVectorParameterValue _returnvalue "AlternateColor" Alternate%20Color :!class /Script/Engine.MaterialInstanceDynamic))