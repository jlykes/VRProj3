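; BP_JumpPickup is a pickup that temporarily changes the jump height of a Character that touches it.
; Overlapping the mesh spawns an explosion effect for any actor, then a Character cast gates hiding the pickup and setting JumpZVelocity to JumpBoostValue.
; After a PowerUpTime delay, it sets the velocity to a hardcoded default rather than the saved original, then destroys itself.
; Collision stays enabled while hidden.
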(event OnComponentBeginOverlap(PickupMesh)
  (params (OtherActor :type Actor%20Object%20Reference) (OtherComp :type Primitive%20Component%20Object%20Reference) (OtherBodyIndex :type Integer) (bFromSweep :type Boolean) (SweepResult :type Hit%20Result%20Structure%20%28by%20ref%29))
  (Effects|SpawnEmitteratLocation "/Game/StarterContent/Particles/P_Explosion.P_Explosion" (Transformation|GetActorLocation))
  (bind _ascharacter (Utilities|Casting|CastToCharacter OtherActor))
  (Rendering|SetActorHiddenInGame true)
  (Variables|/Script/Engine.CharacterMovementComponent|SetJumpZVelocity (Variables|/Script/Engine.Character|GetCharacterMovement _ascharacter) (Variables|Default|GetJumpBoostValue))
  (Utilities|FlowControl|Delay (Variables|Default|GetPowerUpTime))
  (Variables|/Script/Engine.CharacterMovementComponent|SetJumpZVelocity (Variables|/Script/Engine.Character|GetCharacterMovement _ascharacter) 4e+02)
  (Actor|DestroyActor))

(event EventBeginPlay)

(event EventActorBeginOverlap
  (params (OtherActor :type Actor%20Object%20Reference)))

(event EventTick
  (params (DeltaSeconds :type Float%20%28single-precision%29)))

(fn ConstructionScript)