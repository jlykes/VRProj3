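; BP_PlatformForwardMover is a switch actor that moves a linked building block platform forward when its trace-hit event fires.
; The construction script gives the Cone a dynamic material instance with two configurable colors.
; On a hit, a timeline restarts to drive the material's LerpAlpha as visual feedback, then PlatformTarget is cast to BP_BuildingBlockMovable and MoveForward is called without waiting for the timeline.
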(event EventBeginPlay)

(event EventActorBeginOverlap
  (params (OtherActor :type Actor%20Object%20Reference)))

(event EventTick
  (params (DeltaSeconds :type Float%20%28single-precision%29)))

(event EventTraceHitActorwithComponent
  (params (Component :type Primitive%20Component%20Object%20Reference))
  (Utilities|FlowControl|Sequence
    (:then_0
      (bind _alpha (Timeline|AlphaTimeline PlayFromStart)
        (:Update
          (bind _asmaterial_instance_dynamic (Utilities|Casting|CastToMaterialInstanceDynamic (Rendering|Material|GetMaterial (Variables|Default|GetCone) 0)))
          (Rendering|Material|SetScalarParameterValue _asmaterial_instance_dynamic "LerpAlpha" _alpha :!class /Script/Engine.MaterialInstanceDynamic))))
    (:then_1
      (bind _asbp_building_block_movable (Utilities|Casting|CastToBP_BuildingBlockMovable (Variables|Default|GetPlatformTarget)))
      (Default|MoveForward _asbp_building_block_movable))))

(fn ConstructionScript
  (CallFunction|CreateDMI (Variables|Default|GetCone) (Variables|Default|GetColor1) (Variables|Default|GetColor2)))

(fn CreateDMI
  (params (SM :type Static%20Mesh%20Component%20Object%20Reference) (Color :type Linear%20Color%20Structure) (Alternate%20Color :type Linear%20Color%20Structure))
  (bind _returnvalue (Rendering|Material|CreateDynamicMaterialInstance SM 0 (Rendering|Material|GetMaterial SM 0) :!class /Script/Engine.PrimitiveComponent))
  (Rendering|Material|SetVectorParameterValue _returnvalue "BaseColor" Color :!class /Script/Engine.MaterialInstanceDynamic)
  (Rendering|Material|SetVectorParameterValue _returnvalue "AlternateColor" Alternate%20Color :!class /Script/Engine.MaterialInstanceDynamic))