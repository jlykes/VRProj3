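; First-person player character with standard move, look and jump controls plus a reticle-based interaction.
; Holding Interact shows a billboard reticle, which a per-tick camera trace snaps to the surface ahead or the trace's end point.
; Releasing hides it and fires a debug-drawn visibility trace, messaging the hit actor with the component struck.
; A reset input reopens the assignment level and restores the starting transform.
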(event EventBeginPlay
  (Variables|Default|SetOriginalTransform (Transformation|GetActorTransform)))

(event EventActorBeginOverlap
  (params (OtherActor :type Actor%20Object%20Reference)))

(event EventTick
  (params (DeltaSeconds :type Float%20%28single-precision%29))
  ;[1 1 1] Reticle/Raytrace
  (Utilities|FlowControl|Sequence
    (:then_0
      (CallFunction|UpdateReticle))))

(event Input|ActionEvents|InputActionResetToStart
  (:Pressed
    (Game|OpenLevel(byName) "assign3-1")
    (Transformation|SetActorTransform (Variables|Default|GetOriginalTransform))))

(event Input|ActionEvents|InputActionJump
  ;[1 1 1] Movement Controls
  ;;[1 1 1] Jump action
  (:Pressed
    (Character|Jump))
  (:Released
    (Character|StopJumping)))

(event Input|ActionEvents|InputActionInteract
  (bind _camera (Variables|Default|GetCamera))
  (bind _reticlebillboard (Variables|Default|GetReticleBillboard))
  (bind _returnvalue (Transformation|GetWorldLocation _camera))
  ;[1 1 1] Reticle/Raytrace
  (:Pressed
    (Rendering|SetVisibility _reticlebillboard true false))
  (:Released
    (Rendering|SetVisibility _reticlebillboard false false)
    (bind (_outhit _returnvalue_2) (Collision|LineTraceByChannel _returnvalue (+ _returnvalue (* (Math|Vector|GetForwardVector _camera) 5e+03)) "TraceTypeQuery1" false 0 "ForDuration"))
    (if _returnvalue_2
      (Class|BPIUseInterface|TraceHitActorwithComponent(Message) (.HitActor (Collision|BreakHitResult _outhit)) (.HitComponent (Collision|BreakHitResult _outhit))))))

(event Input|AxisEvents|InputAxisTurn
  (params (AxisValue :type Float%20%28single-precision%29))
  ;[1 1 1] Movement Controls
  ;;[1 1 1] Turn Left and Right With Mouse
  (Pawn|Input|AddControllerYawInput AxisValue))

(event Input|AxisEvents|InputAxisMoveForward
  (params (AxisValue :type Float%20%28single-precision%29))
  ;[1 1 1] Movement Controls
  ;;[1 1 1] Move Forward/Right
  (Pawn|Input|AddMovementInput (Transformation|GetActorForwardVector) AxisValue false))

(event Input|AxisEvents|InputAxisLookUpRate
  (params (AxisValue :type Float%20%28single-precision%29))
  ;[1 1 1] Movement Controls
  ;;[1 1 1] Look up and down with rate
  (Pawn|Input|AddControllerPitchInput (* AxisValue (Utilities|Time|GetWorldDeltaSeconds) (Variables|Default|GetLookUpRateScalar))))

(event Input|AxisEvents|InputAxisLookUp
  (params (AxisValue :type Float%20%28single-precision%29))
  ;[1 1 1] Movement Controls
  ;;[1 1 1] Look up
  (Pawn|Input|AddControllerPitchInput AxisValue))

(event Input|AxisEvents|InputAxisMoveRight
  (params (AxisValue :type Float%20%28single-precision%29))
  ;[1 1 1] Movement Controls
  ;;[1 1 1] Move Forward/Right
  (Pawn|Input|AddMovementInput (Transformation|GetActorRightVector) AxisValue false))

(event Input|AxisEvents|InputAxisTurnRate
  (params (AxisValue :type Float%20%28single-precision%29))
  ;[1 1 1] Movement Controls
  ;;[1 1 1] Turn Left/Right With Keyboard
  (Pawn|Input|AddControllerYawInput (* AxisValue (Utilities|Time|GetWorldDeltaSeconds) (Variables|Default|GetTurnRateScalar))))

(fn ConstructionScript)

(fn UpdateReticle
  (bind (_startpoint _endpoint) (Utilities|ReticlePoints))
  (bind (_outhit _returnvalue) (Collision|LineTraceByChannel _startpoint _endpoint "TraceTypeQuery1" false 0 "None"))
  (if _returnvalue
    (LocalVariables|SetReticleLocation (.Location (Collision|BreakHitResult _outhit)))
    (else
      (LocalVariables|SetReticleLocation (.EndPoint (Utilities|ReticlePoints)))))
  (Transformation|SetWorldLocation (Variables|Default|GetReticleBillboard) (LocalVariables|GetReticleLocation) false))