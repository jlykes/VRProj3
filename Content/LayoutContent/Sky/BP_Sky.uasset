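; BP_Sky is a sky Blueprint that colors a Sky component with adjustable material settings.
; Its construction script creates a dynamic instance of M_Sky on the first material slot and stores it as SkyMaterial.
; It then passes four color variables, plus Horizon and ColorValue scalars, into that instance, so the look is applied at construction with no runtime logic shown.
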(fn ConstructionScript
  (Utilities|FlowControl|Sequence
    (:then_0
      (bind _returnvalue (Rendering|Material|CreateDynamicMaterialInstance (Variables|Default|GetSky) 0 "/Game/LayoutContent/Sky/M_Sky.M_Sky" :!class /Script/Engine.PrimitiveComponent))
      (Variables|Default|SetSkyMaterial _returnvalue))
    (:then_1
      (Rendering|Material|SetVectorParameterValue (Variables|Default|GetSkyMaterial) "ColorA" (Variables|Default|GetColorA) :!class /Script/Engine.MaterialInstanceDynamic))
    (:then_2
      (Rendering|Material|SetVectorParameterValue (Variables|Default|GetSkyMaterial) "ColorB" (Variables|Default|GetColorB) :!class /Script/Engine.MaterialInstanceDynamic))
    (:then_3
      (Rendering|Material|SetVectorParameterValue (Variables|Default|GetSkyMaterial) "ColorC" (Variables|Default|GetColorC) :!class /Script/Engine.MaterialInstanceDynamic))
    (:then_4
      (Rendering|Material|SetVectorParameterValue (Variables|Default|GetSkyMaterial) "ColorD" (Variables|Default|GetColorD) :!class /Script/Engine.MaterialInstanceDynamic))
    (:then_5
      (Rendering|Material|SetScalarParameterValue (Variables|Default|GetSkyMaterial) "Horizon" (Variables|Default|GetHorizon) :!class /Script/Engine.MaterialInstanceDynamic))
    (:then_6
      (Rendering|Material|SetScalarParameterValue (Variables|Default|GetSkyMaterial) "ColorValue" (Variables|Default|GetColorValue) :!class /Script/Engine.MaterialInstanceDynamic))))